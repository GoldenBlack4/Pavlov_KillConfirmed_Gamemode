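; Player proxy for the Kill Confirmed custom mode that backs up each player's loadout.
; In game modes named "Custom…", it caches player state and snapshots inventory, held items, attachments, cash, score and skin into CMP_KC_PlayerInfo on a looping timer.
; Death shortens pawn lifespan and, in those modes, stops the timer.
; SpawnDogtag can spawn a team-tagged KC_DogTag, but nothing in this Blueprint calls it.
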(event `OnBeginPlay`
  ;[1 1 1] Kill Confirmed
  ;;[1 1 1] Begin Play
  (`KismetSystemLibrary.Delay` 1.0)
  (`self.SetTimerLoadout`)
  (bind (_playerstatus _bsucceeded) (`PavlovProxyStatics.GetPavlovPlayerStatusByPawn` (`self.GetPawn`)))
  (if _bsucceeded
    (bind _output_get (set `self.PlayerState` (break `PavlovPlayerStatus` _playerstatus)))
    (set `self.PlayerName` (`PlayerState.GetPlayerName` _output_get))
    (set `self.PlayerTeamID` (`.TeamId` (break `PavlovPlayerStatus` _playerstatus)))
    (bind _ascmp_kc_player_info (cast `/Game/CustomMaps/KILLCONFIRMED/CMP_KC_PlayerInfo` (`Pavlov_Library.GetPlayerInfo` (`self.PlayerState`))))
    (set `self.PlayerInfoRef` _ascmp_kc_player_info)))

(event `self.ReceiveBeginPlay`
  ;[1 1 1] Kill Confirmed
  ;;[1 1 1] Begin Play
  (if (`KismetStringLibrary.StartsWith` (`KismetSystemLibrary.GetDisplayName` (`GameplayStatics.GetGameMode`)) "Custom")
    (`self.OnBeginPlay`)))

(event `SetTimerLoadout`
  ;[1 1 1] Kill Confirmed
  ;;[0.5884 1 0.3767] Save Loadout
  (bind _returnvalue (`KismetSystemLibrary.K2_SetTimerDelegate` (delegate `SaveLoadout`) 1.0 true))
  (set `self.TimerHandle` _returnvalue))

(event `SaveLoadout`
  (bind _playerinforef (`self.PlayerInfoRef`))
  ;[1 1 1] Kill Confirmed
  ;;[0.5884 1 0.3767] Save Loadout
  (`/Game/CustomMaps/KILLCONFIRMED/CMP_KC_PlayerInfo.ClearLoadoutArray` (`self.PlayerInfoRef`))
  (bind _invitems (`self.GetAllInventoryItems`))
  (bind _output_get (set `self.Inventory` _invitems))
  (for _array_element _output_get
    (bind (_attachments _returnvalue) (`self.GetWeaponAttachments` (`.Item` (break `InventoryItem` _array_element))))
    (if _returnvalue
      (set `self.InventoryAttachments` _attachments)))
  (bind (_bhasitem _item) (`self.GetHeldItem` true))
  (bind _attachments_2 (`self.GetWeaponAttachments` (`.Item` (break `PlayerItem` _item))))
  (set `self.DominantAttachments` _attachments_2)
  (bind (_bhasitem_2 _item_2) (`self.GetHeldItem` false))
  (bind _attachments_3 (`self.GetWeaponAttachments` (`.Item` (break `PlayerItem` _item_2))))
  (set `self.NonDominantAttachments` _attachments_3)
  (bind _playerstatus (`PavlovProxyStatics.GetPavlovPlayerStatus` (`self.PlayerState`)))
  (`/Game/CustomMaps/KILLCONFIRMED/CMP_KC_PlayerInfo.SaveLoadout` (`self.PlayerInfoRef`) (`self.Inventory`) _item _item_2 (`.Cash` (break `PavlovPlayerStatus` _playerstatus)) (`.Score` (break `PavlovPlayerStatus` _playerstatus)) (`self.InventoryAttachments`) (`self.DominantAttachments`) (`self.NonDominantAttachments`))
  (`/Game/CustomMaps/KILLCONFIRMED/CMP_KC_PlayerInfo.SetSkin` _playerinforef (`self.GetPlayerSkin`))
  (`/Game/CustomMaps/KILLCONFIRMED/CMP_KC_PlayerInfo.SetLoadOutSaved` _playerinforef))

(event `self.OnSkinChanged`
  (params (Skin :type Name))
  ;[1 1 1] Kill Confirmed
  ;;[0.5884 1 0.3767] Save Loadout
  (`/Game/CustomMaps/KILLCONFIRMED/CMP_KC_PlayerInfo.SetSkin` (`self.PlayerInfoRef`) Skin))

(event `OnDeath`
  (params (KilledActor :type "Actor Object Reference"))
  ;[1 1 1] Kill Confirmed
  ;;[1 0.2917 0.2917] Spawn Dogtag
  (`KismetSystemLibrary.K2_ClearAndInvalidateTimerHandle` (`self.TimerHandle`)))

(event `self.OnPlayerDeath`
  (params (KilledActor :type "Actor Object Reference"))
  ;[1 1 1] Kill Confirmed
  ;;[1 0.2917 0.2917] Spawn Dogtag
  (`self.SetLifeSpan` (`self.GetPawn`) 10.0)
  (if (`KismetStringLibrary.StartsWith` (`KismetSystemLibrary.GetDisplayName` (`GameplayStatics.GetGameMode`)) "Custom")
    (`self.OnDeath` KilledActor)))

(fn `GetVoiceAttenuation`
  (returns (ReturnValue :type "SoundAttenuation Object Reference"))
  ;[1 1 1] Set attenuation here
  (return null))

(fn `SpawnDogtag`
  (params (KilledActor :type "Actor Object Reference"))
  (`|SpawnActorFromClass` "/Game/CustomMaps/KILLCONFIRMED/DogTag/KC_DogTag.KC_DogTag_C" (`self.GetTransform` KilledActor) "AlwaysSpawn" "OverrideRootScale" null (`self.PlayerTeamID`) (`self.PlayerName`) 20.0 "/Game/CustomMaps/KILLCONFIRMED/DogTag/Sounds/kill_confirmed_bo2.kill_confirmed_bo2" "/Game/CustomMaps/KILLCONFIRMED/DogTag/Sounds/KC_Removed.KC_Removed" (`self.PlayerState`) false 0 "KillerName" null))

(fn `UserConstructionScript`)