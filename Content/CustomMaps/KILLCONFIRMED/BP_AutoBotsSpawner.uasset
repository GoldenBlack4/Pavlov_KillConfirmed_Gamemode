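; BP_AutoBotsSpawner keeps a Pavlov custom-mode map stocked with AI bots, destroying itself on the server in other game modes.
; Once the round leaves its starting or standby state, a server loop counts bots and humans from the PlayerArray, spawning pawns until the target is met.
; Spawning pauses when humans exceed a cap or Remove is pressed.
; Server-replicated buttons add a bot and resume spawning, or clear all bots.
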(event `self.ReceiveBeginPlay`
  (bind _state (`Pavlov_GameLogic.GetRoundState` (`Pavlov_Library.GetGameLogic`)))
  ;[1 1 1] Begin Play waiting
  (`KismetSystemLibrary.Delay` 1.0)
  (`/Engine/EditorBlueprintResources/ActorMacros.Switch Has Authority` :!label _label
    (:`Authority`
      (if (`KismetStringLibrary.StartsWith` (`KismetSystemLibrary.GetDisplayName` (`GameplayStatics.GetGameMode`)) "Custom")
        (if (or (`|EnumEquality` _state "Starting") (`|EnumEquality` _state "StandBy"))
          (`KismetSystemLibrary.Delay` 1.0)
          (goto _label)
          (else
            (`self.SpawnLoop`)))
        (else
          (`self.K2_DestroyActor`))))))

(event `SpawnLoop`
  ;[1 1 1] Calculate if bot is needed
  (set `self.AliveBotsCount` 0)
  (set `self.NumOfPlayers` 0)
  (if (== (`self.NeededBotsCount`) 0)
    (`self.K2_DestroyActor`)
    (else
      (bind _asgame_state (cast `GameState` (`GameplayStatics.GetGameState`)))
      (for _array_element (`GameStateBase.PlayerArray` _asgame_state)
        (bind _playerstatus (`PavlovProxyStatics.GetPavlovPlayerStatus` _array_element))
        (bind _playerstate (break `PavlovPlayerStatus` _playerstatus))
        (`/Engine/EditorBlueprintResources/StandardMacros.IsValid` _playerstate
          (:`Is Valid`
            (if (`PlayerState.bIsABot` _playerstate)
              (`/Engine/EditorBlueprintResources/StandardMacros.IncrementInt` (`self.AliveBotsCount`))
              (else
                (`/Engine/EditorBlueprintResources/StandardMacros.IncrementInt` (`self.NumOfPlayers`)))))))
      (if (>= (`self.AliveBotsCount`) (`self.NeededBotsCount`))
        (`KismetSystemLibrary.Delay` 1.0 :!label _label_2)
        (`self.SpawnLoop`)
        (elif (> (`self.NumOfPlayers`) 8)
          (goto _label_2)
          (elif (`self.StopBotsSpawning`)
            (goto _label_2)
            (else
              (`self.SpawnBot`))))))))

(event `SpawnBot`
  ;[0.4305 1 0.5236] Spawn a bot
  (`AIBlueprintHelperLibrary.SpawnAIFromClass` "/Game/Gameplay/BP_PavlovPawn.BP_PavlovPawn_C" null (`self.K2_GetActorLocation`) (struct) true)
  (`KismetSystemLibrary.Delay` (`self.LoopDelay`))
  (`self.SpawnLoop`))

(event `self.Pavlov_AddButton.OnInteractBoxClient`
  (params (InteractType :type "EInteractType Enum" :default "Grabbed") (HandProxy :type "Pavlov_HandProxy Object Reference") (InteractBox :type "Pavlov_InteractBox Object Reference"))
  ;[1 1 1] Replicate
  (`Pavlov_HandProxy.ReplicateInteract_Server` HandProxy InteractType InteractBox))

(event `self.Pavlov_RemoveButton.OnInteractBoxClient`
  (params (InteractType :type "EInteractType Enum" :default "Grabbed") (HandProxy :type "Pavlov_HandProxy Object Reference") (InteractBox :type "Pavlov_InteractBox Object Reference"))
  ;[1 1 1] Replicate
  (`Pavlov_HandProxy.ReplicateInteract_Server` HandProxy InteractType InteractBox))

(event `self.Pavlov_AddButton.OnInteractBoxServer`
  (params (InteractType :type "EInteractType Enum" :default "Grabbed") (HandProxy :type "Pavlov_HandProxy Object Reference") (InteractBox :type "Pavlov_InteractBox Object Reference"))
  ;[0.4305 1 0.5236] Spawn a bot
  (`AIBlueprintHelperLibrary.SpawnAIFromClass` "/Game/Gameplay/BP_PavlovPawn.BP_PavlovPawn_C" null (`self.K2_GetActorLocation`) (struct) true)
  (set `self.StopBotsSpawning` false))

(event `self.Pavlov_RemoveButton.OnInteractBoxServer`
  (params (InteractType :type "EInteractType Enum" :default "Grabbed") (HandProxy :type "Pavlov_HandProxy Object Reference") (InteractBox :type "Pavlov_InteractBox Object Reference"))
  ;[1 0.1765 0.1666] Remove all bots
  (bind _outactors (`GameplayStatics.GetAllActorsOfClass` "/Game/Gameplay/BP_PavlovPawn.BP_PavlovPawn_C"))
  (bind (_arrayindex _arrayelement) (`/Engine/EditorBlueprintResources/StandardMacros.ReverseForEachLoop` _outactors)
    (:`LoopBody`
      (if (not (`Pawn.IsPlayerControlled` _arrayelement))
        (`self.K2_DestroyActor` _arrayelement)))
    (:`Completed`
      (bind _outactors_2 (`GameplayStatics.GetAllActorsOfClass` "/Script/Engine.PlayerState"))
      (for _array_element _outactors_2
        (if (`PlayerState.bIsABot` _array_element)
          (`self.K2_DestroyActor` _array_element)))
      (set `self.AliveBotsCount` 0)
      (set `self.StopBotsSpawning` true))))

(fn `UserConstructionScript`)